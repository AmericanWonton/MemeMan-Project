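; HUD Blueprint that owns the game's widgets: stamina/score/timer display, QTE questions, pause menu and game over screen.
; Tick uses a Delay to count the capped timer down each second, updating score and triggering BP_CaptainWinState at zero.
; QTEs hide the timer display, then rebuild a shuffled question batch when answered.
; Pausing hides or restores widgets and their animations through the BPI_HideableWidgets interface.
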(event `self.ReceiveBeginPlay`
  (bind _user_widget_arrays (`self.User Widget Arrays`))
  ;[1 1 1] USed to add the QTE Widgets we create
  (bind _returnvalue (`|CreateWidget` "/Game/Widgets/W_QTEQuestion1.W_QTEQuestion1_C"))
  (`KismetArrayLibrary.Array_Add` _user_widget_arrays _returnvalue)
  (bind _returnvalue_2 (`|CreateWidget` "/Game/Widgets/W_QTEQuestion2.W_QTEQuestion2_C"))
  (`KismetArrayLibrary.Array_Add` _user_widget_arrays _returnvalue_2))

(event `Player Creator`
  ;[1 1 1] Set Widget and Character Reference
  (bind _outactors (`GameplayStatics.GetAllActorsOfClass` "/Game/ThirdPersonBP/Blueprints/BP_MemeMan.BP_MemeMan_C"))
  (set `self.Meme Man Referenc` (`|GetArrayItem` _outactors)))

(event `Time Decreaser`
  ;[1 1 1] Increase or Decrease Timer
  (set `self.Timer Value` (- (`self.Timer Value`) 30.0)))

(event `Hud Creator`
  ;[1 1 1] Set Widget and Character Reference
  (bind _returnvalue (`|CreateWidget` "/Game/Widgets/w_basicStaminaScoreandTimer.w_basicStaminaScoreandTimer_C"))
  (bind _output_get (set `self.Timer Reference` _returnvalue))
  (`UserWidget.AddToViewport` _output_get 0))

(event `Create Batch of QTE Widgets`
  (bind _user_widget_arrays (`self.User Widget Arrays`))
  ;[1 1 1] Kill and Create a batch of widgets
  (`KismetArrayLibrary.Array_Clear` _user_widget_arrays)
  (bind _returnvalue (`|CreateWidget` "/Game/Widgets/W_QTEQuestion1.W_QTEQuestion1_C"))
  (`KismetArrayLibrary.Array_Add` _user_widget_arrays _returnvalue)
  (bind _returnvalue_2 (`|CreateWidget` "/Game/Widgets/W_QTEQuestion2.W_QTEQuestion2_C"))
  (`KismetArrayLibrary.Array_Add` _user_widget_arrays _returnvalue_2)
  (`KismetArrayLibrary.Array_Shuffle` _user_widget_arrays))

(event `Time Increaser`
  ;[1 1 1] Increase or Decrease Timer
  (set `self.Timer Value` (+ (`self.Timer Value`) 30.0)))

(event `self.ReceiveTick`
  (params (DeltaSeconds :type "Float (single-precision)"))
  (bind _meme_man_referenc (`self.Meme Man Referenc`))
  (bind _timer_reference (`self.Timer Reference`))
  ;[1 1 1] Test Timer
  (if (`self.Loaded into Playable Map`)
    (if (<= (`self.Timer Value`) 0.0)
      (set `self.Timer Value` 0.0)
      (`/Engine/EditorBlueprintResources/StandardMacros.DoOnce` false
        (:`Completed`
          ;[1 1 1] Lose State in BP_CaptainWinState
          (bind _outactors (`GameplayStatics.GetAllActorsOfClass` "/Game/BluePrints/BP_CaptainWinState.BP_CaptainWinState_C"))
          (`/Game/BluePrints/BP_CaptainWinState.Win State Shower` (`|GetArrayItem` _outactors))))
      (elif (> (`self.Timer Value`) 90.0)
        (set `self.Timer Value` 90.0)
        (else
          (`KismetSystemLibrary.Delay` 1.0)
          (set `self.Timer Value` (- (`self.Timer Value`) 1.0))
          (`/Game/Widgets/w_basicStaminaScoreandTimer.Timer Setter` _timer_reference (`self.Timer Value`))
          (`/Game/Widgets/w_basicStaminaScoreandTimer.Set Player Score` _timer_reference (`self.Timer Score Adder`))
          (if (`KismetSystemLibrary.IsValid` _meme_man_referenc)
            (`/Game/ThirdPersonBP/Blueprints/BP_MemeMan.Set Player Score` _meme_man_referenc (`self.Timer Score Adder`))))))))

(event `Set Score Widget`
  (params (Amount :type "Float (double-precision)"))
  ;[1 1 1] Set Widget Score
  (`/Game/Widgets/w_basicStaminaScoreandTimer.Set Player Score` (`self.Timer Reference`) Amount))

(event `Speed Do-er`
  (params (`Current Speed` :type "Float (double-precision)"))
  ;[1 1 1] Speed Setter Text
  (if (`self.Loaded into Playable Map`)
    (`/Game/Widgets/w_basicStaminaScoreandTimer.Set Speed Txt` (`self.Timer Reference`) `Current Speed`)))

(event `Player Score Setter`
  (params (PlayerScoreAMNT :type "Float (double-precision)"))
  ;[1 1 1] Set PlayerSCore
  (`/Game/ThirdPersonBP/Blueprints/BP_MemeMan.Set Player Score` (`self.Meme Man Referenc`) PlayerScoreAMNT))

(event `Pause Menu`
  ;[1 1 1] Used to Pause the Game and Stop Ongoing Widgets
  ;;[1 1 1] To Pause
  ;;[1 1 1] Finds all Widgets and Stops Animations in them.
  (bind _foundwidgets (`WidgetBlueprintLibrary.GetAllWidgetsWithInterface` "/Game/Interfaces/BPI_HideableWidgets.BPI_HideableWidgets_C"))
  (for _array_element _foundwidgets :!label _label
    (`Widget.SetVisibility` _array_element "Hidden")
    (message `/Game/Interfaces/BPI_HideableWidgets.Hide Widgets, Stop Anims` _array_element))
  ;;[1 1 1] Adds Pause Menu to Viewport
  (`UserWidget.AddToViewport` (`self.Pause Menu Reference`) 0))

(event `Stop Find Widgets Loop`
  ;[1 1 1] Used to Pause the Game and Stop Ongoing Widgets
  ;;[1 1 1] Finds all Widgets and Stops Animations in them.
  (goto _label :!via `Break`))

(event `Create Pause Menu Ref`
  ;[1 1 1] Creates Pause Menu for Use later
  (bind _returnvalue (`|CreateWidget` "/Game/Widgets/W_PauseMenu.W_PauseMenu_C"))
  (set `self.Pause Menu Reference` _returnvalue))

(event `UnPause Menu`
  ;[1 1 1] Used to Pause the Game and Stop Ongoing Widgets
  ;;[1 1 1] To Un-Pause
  ;;[1 1 1] Resumes all Widget Actions
  (bind _foundwidgets (`WidgetBlueprintLibrary.GetAllWidgetsWithInterface` "/Game/Interfaces/BPI_HideableWidgets.BPI_HideableWidgets_C"))
  (for _array_element _foundwidgets
    (`Widget.SetVisibility` _array_element "Visible")
    (message `/Game/Interfaces/BPI_HideableWidgets.Show Widgets, Reume Anims` _array_element))
  ;;[1 1 1] Gets Rid of Pause Menu
  (`Widget.RemoveFromParent` (`self.Pause Menu Reference`))
  (set `self.Pause Menu Reference` null))

(event `Game Over Widget Creation`
  (params (`Memes Missed` :type Integer) (`Time Left` :type "Float (double-precision)") (`Won or Lost` :type Boolean))
  ;[1 1 1] Creates Game Over Widget and sets Variables for the SCoreboard
  (`WidgetLayoutLibrary.RemoveAllWidgets`)
  (bind _returnvalue (`|CreateWidget` "/Game/Widgets/W_GameOver.W_GameOver_C"))
  (`/Game/Widgets/W_GameOver.Set Win State` _returnvalue `Won or Lost`)
  (`/Game/Widgets/W_GameOver.Set Meme Amount` _returnvalue `Memes Missed`)
  (`/Game/Widgets/W_GameOver.Set Time Amount` _returnvalue `Time Left`)
  (`/Game/Widgets/W_GameOver.Set Final Score` _returnvalue (`self.Player Final Score`))
  (`UserWidget.AddToViewport` _returnvalue 0))

(event `Add new QTE Widget`
  (params (`Which One?` :type Integer))
  ;[1 1 1] Do the QTE, add the Widget, and remove it once player wins/loses
  (bind _what_widget (`self.Which Widget to Add?` `Which One?`)
    (:`Adding Widget1`
      (`Widget.SetVisibility` (`self.Timer Reference`) "Hidden")
      (set `self.Current QTE Widget` _what_widget)
      (`UserWidget.AddToViewport` (`|GetArrayItem` (`self.User Widget Arrays`) _what_widget) 0))
    (:`Adding Widget 2`
      (`Widget.SetVisibility` (`self.Timer Reference`) "Hidden")
      (set `self.Current QTE Widget` _what_widget)
      (`UserWidget.AddToViewport` (`|GetArrayItem` (`self.User Widget Arrays`) _what_widget) 0))))

(event `Correct Ansewer!`
  (params (`Won or lost` :type Boolean))
  ;[1 1 1] Do the QTE, add the Widget, and remove it once player wins/loses
  (`Widget.RemoveFromParent` (`|GetArrayItem` (`self.User Widget Arrays`) (`self.Current QTE Widget`)))
  (`Widget.SetVisibility` (`self.Timer Reference`) "Visible")
  (`self.Create Batch of QTE Widgets`))

(event `Incorrect Ansewer`
  (params (`Won or Lost` :type Boolean))
  ;[1 1 1] Do the QTE, add the Widget, and remove it once player wins/loses
  (`Widget.RemoveFromParent` (`|GetArrayItem` (`self.User Widget Arrays`) (`self.Current QTE Widget`)))
  (`Widget.SetVisibility` (`self.Timer Reference`) "Visible")
  (`self.Create Batch of QTE Widgets`))

(fn `UserConstructionScript`)