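; BP_ThePlayerController is the game's player controller, handling possession, camera blends and input modes for QTEs, lava deaths, game over and pausing.
; QTE and game over events possess the target actor and blend the view to it, and the QTE exit re-possesses BP_MemeMan.
; Lava death hides and disables the character during a timed lava-camera shot, then restores it.
; Pause and QTE control events toggle the cursor between UI-only and game-only input.
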(event `take away Controls for QTE`
  ;[1 1 1] Takes away mouse input and controls
  (set `self.bShowMouseCursor` false)
  (`WidgetBlueprintLibrary.SetInputMode_GameOnly` self))

(event `Game Over Camera`
  (params (`CaptainWinState Ref` :type "/Game/BluePrints/BP_CaptainWinState_Camera Object Reference"))
  ;[1 1 1] Game Over Camera
  (`self.Possess` `CaptainWinState Ref`)
  (`self.Allow Controls for QTE`)
  (`self.SetViewTargetWithBlend` `CaptainWinState Ref` 5.0 "VTBlend_EaseOut"))

(event `Allow Controls for QTE`
  ;[1 1 1] Allows for mouse controls to select input (May not need for phones)
  (set `self.bShowMouseCursor` true)
  (`WidgetBlueprintLibrary.SetInputMode_UIOnlyEx` self null))

(event `QTE Event`
  (params (`Which QTE?` :type "/Game/BluePrints/BP_QTEPawn Object Reference"))
  ;[1 1 1] QTE Transition
  (`KismetSystemLibrary.PrintString` "Possessing QTE Actor!")
  (`self.Possess` `Which QTE?`)
  (`self.SetViewTargetWithBlend` `Which QTE?` 1.0 "VTBlend_EaseIn"))

(event `Dead Respawn!`
  (params (`The Lava Camera` :type "/Game/BluePrints/BP_NotLav Object Reference"))
  ;[1 1 1] Lava hide then respawn
  (bind _outactors (`GameplayStatics.GetAllActorsOfClass` "/Game/ThirdPersonBP/Blueprints/BP_MemeMan.BP_MemeMan_C"))
  (bind _output (`|GetArrayItem` _outactors))
  (`self.SetActorHiddenInGame` _output true)
  (`self.DisableInput` _output self)
  (`self.SetViewTargetWithBlend` `The Lava Camera` 1.0 "VTBlend_EaseIn")
  (`KismetSystemLibrary.Delay` 3.0)
  (`self.SetActorHiddenInGame` _output false)
  (`self.EnableInput` _output self)
  (`self.SetViewTargetWithBlend` _output 1.0))

(event `QTE Exit Transition`
  ;[1 1 1] QTE Exit
  (`KismetSystemLibrary.PrintString` "Possesing Character Again!")
  (bind _outactors (`GameplayStatics.GetAllActorsOfClass` "/Game/ThirdPersonBP/Blueprints/BP_MemeMan.BP_MemeMan_C"))
  (`self.Possess` (`|GetArrayItem` _outactors)))

(event `Pause Game MOvement`
  ;[1 1 1] Used to Pause and Unpause Player Movement for the Game
  (set `self.bShowMouseCursor` true)
  (bind _asbp_the_hud (cast `/Game/Utility/BP_TheHUD` (`self.GetHUD` self))
    (:`then`
      (`WidgetBlueprintLibrary.SetInputMode_UIOnlyEx` self (`/Game/Utility/BP_TheHUD.Pause Menu Reference` _asbp_the_hud)))
    (:`CastFailed`
      (`KismetSystemLibrary.PrintString` "Cast failed in BP_PlayerControoller for BP_The HUDo"))))

(event `UnPause Game Movement`
  ;[1 1 1] Used to Pause and Unpause Player Movement for the Game
  (set `self.bShowMouseCursor` false)
  (`WidgetBlueprintLibrary.SetInputMode_GameOnly` self))

(fn `UserConstructionScript`)