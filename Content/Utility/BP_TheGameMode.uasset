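; Game mode that boots the playable-map HUD and persists per-level high scores in a save game.
; BeginPlay loads or creates the score slot, and a separate event has BP_TheHUD create the HUD and player.
; SaveandLoadPlayerScore routes by level through the WhatLVL2Save macro, with only level 1 implemented.
; An existing save's score is overwritten unconditionally; only a newly created save compares scores first.
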(event `Load "Playing HUD"`
  ;[1 1 1] Activates the Timer
  (bind _asbp_the_hud (cast `/Game/Utility/BP_TheHUD` (`PlayerController.GetHUD` (`GameplayStatics.GetPlayerController` 0)))
    (:`then`
      (set `/Game/Utility/BP_TheHUD.Loaded into Playable Map` true _asbp_the_hud)
      (`/Game/Utility/BP_TheHUD.Hud Creator` _asbp_the_hud)
      (`/Game/Utility/BP_TheHUD.Player Creator` _asbp_the_hud))
    (:`CastFailed`
      (`KismetSystemLibrary.PrintString` "Cast failed to BP_THe Hud in BP_TheGameMode"))))

(event `self.ReceiveBeginPlay`
  ;[1 1 1] Creatres Save Games for Players to use later
  ;;[1 1 1] Check to see if Scores Exist
  (bind _returnvalue (`GameplayStatics.DoesSaveGameExist` (`self.HS_SaveSlots`)))
  (if _returnvalue
    ;;[1 1 1] Loading High Scores
    (bind _returnvalue_2 (`GameplayStatics.LoadGameFromSlot` (`self.HS_SaveSlots`)))
    (bind _asbp_save_game (cast `/Game/BluePrints/SaveGame_and_HighScores/BP_SaveGame` _returnvalue_2)
      (:`then`
        (set `self.SaveGameRef` _asbp_save_game)
        (`KismetSystemLibrary.PrintString` "Loaded Last Times HS" true true (struct :`R` 1.0 :`G` 0.053581 :`A` 1.0) 4.0))
      (:`CastFailed`
        (`KismetSystemLibrary.PrintString` "Cast failed to BP_SaveGagme in BP_TheGagmeMode")))
    (else
      ;;[1 1 1] Creates Save Game if there isn't
      (bind _returnvalue_3 (`GameplayStatics.CreateSaveGameObject` "/Game/BluePrints/SaveGame_and_HighScores/BP_SaveGame.BP_SaveGame_C"))
      (bind _output_get (set `self.SaveGameRef` _returnvalue_3))
      (`GameplayStatics.SaveGameToSlot` _output_get (`self.HS_SaveSlots`))
      (`KismetSystemLibrary.PrintString` (`KismetStringLibrary.Concat_StrStr` "High Scores Saved!") true true (struct :`G` 0.092447 :`B` 1.0 :`A` 1.0) 4.0))))

(event `Save and Load Player Score`
  (params (Score :type "Float (double-precision)") (`What Level?` :type Text))
  ;[1 1 1] Sets Player Score when Game is Over
  ;;[1 1 1] Check to see if Scores Exist
  (bind _returnvalue (`GameplayStatics.DoesSaveGameExist` (`self.HS_SaveSlots`)))
  (if _returnvalue
    ;[1 1 1] Loading High Scores
    (bind _returnvalue_2 (`GameplayStatics.LoadGameFromSlot` (`self.HS_SaveSlots`)))
    (bind _asbp_save_game (cast `/Game/BluePrints/SaveGame_and_HighScores/BP_SaveGame` _returnvalue_2)
      (:`then`
        (bind _output_get (set `self.SaveGameRef` _asbp_save_game))
        ;[1 1 1] Savings High Scores(LVL1)
        (`self.What LVL 2 Save?` `What Level?`
          (:`Lvl 1`
            (bind (_level1score _level2score _level3score _level4score _level5score) (break `/Game/BluePrints/SaveGame_and_HighScores/SaveSTRT` (`/Game/BluePrints/SaveGame_and_HighScores/BP_SaveGame.Level HighScores` _output_get)))
            (set `/Game/BluePrints/SaveGame_and_HighScores/BP_SaveGame.Level HighScores` (make `/Game/BluePrints/SaveGame_and_HighScores/SaveSTRT` Score _level2score _level3score _level4score _level5score) _output_get)
            (bind _output_get_2 (set `self.SaveGameRef` _output_get))
            (`GameplayStatics.SaveGameToSlot` _output_get_2 (`self.HS_SaveSlots`))
            (`KismetSystemLibrary.PrintString` (`KismetStringLibrary.Concat_StrStr` "High Scores Saved!" " ALthough now we aded a score!") true true (struct :`R` 1.0 :`G` 0.574923 :`A` 1.0) 4.0))
          (:`Other LVLS...`
            (`KismetSystemLibrary.PrintString` "We got no other levels yet, chief"))))
      (:`CastFailed`
        (`KismetSystemLibrary.PrintString` "Cast failed to BP_SaveGagme in BP_TheGagmeMode")))
    (else
      ;;[1 1 1] Savings High Scores(LVL1)
      (bind _returnvalue_3 (`GameplayStatics.CreateSaveGameObject` "/Game/BluePrints/SaveGame_and_HighScores/BP_SaveGame.BP_SaveGame_C"))
      (`self.What LVL 2 Save?` `What Level?`
        (:`Lvl 1`
          (bind (_level1score_2 _level2score_2 _level3score_2 _level4score_2 _level5score_2) (break `/Game/BluePrints/SaveGame_and_HighScores/SaveSTRT` (`/Game/BluePrints/SaveGame_and_HighScores/BP_SaveGame.Level HighScores` _returnvalue_3)))
          ;;;[1 1 1] If LVL1 Score Better or Not
          (if (>= Score _level1score_2)
            (set `/Game/BluePrints/SaveGame_and_HighScores/BP_SaveGame.Level HighScores` (make `/Game/BluePrints/SaveGame_and_HighScores/SaveSTRT` Score _level2score_2 _level3score_2 _level4score_2 _level5score_2) _returnvalue_3)
            (bind _output_get_3 (set `self.SaveGameRef` _returnvalue_3))
            (`GameplayStatics.SaveGameToSlot` _output_get_3 (`self.HS_SaveSlots`))
            (`KismetSystemLibrary.PrintString` (`KismetStringLibrary.Concat_StrStr` "High Scores Saved!"))))
        (:`Other LVLS...`
          (`KismetSystemLibrary.PrintString` "We got no other levels yet, chief"))))))

(fn `UserConstructionScript`)