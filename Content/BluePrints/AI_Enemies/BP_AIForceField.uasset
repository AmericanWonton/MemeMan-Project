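; AI forcefield enemy that chases the player's BP_MemeMan while it is possessed and gets knocked away after a completed QTE.
; Tick rotates it toward the player and moves it forward, or fires a do-once knockback when GettingKnocked is set.
; A timeline lerps it to the BP_ForcefieldKnockbackDirector's transform, then clears the flag and re-arms.
; SpeedDoer uses one-shot timelines to raise floating-movement max speed at PlayerScore thresholds.
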(event `Knock ForceField`
  ;[1 1 1] If QTE Complete, "GettingKnocked" == True and we send the Forcefeild flying
  (`KismetSystemLibrary.PrintString` "Calling Knock FOrcefield")
  (bind _outactors (`GameplayStatics.GetAllActorsOfClass` "/Game/BluePrints/BP_ForcefieldKnockbackDirector.BP_ForcefieldKnockbackDirector_C"))
  (bind (_direction _time2move) (`Timeline|BP_Forcefield Mover` :!via `PlayFromStart`)
    (:`Update`
      (bind _output (`|GetArrayItem` _outactors))
      (`self.K2_SetActorLocationAndRotation` (`KismetMathLibrary.VLerp` (`self.K2_GetActorLocation` self) (`self.K2_GetActorLocation` _output) _time2move) (`self.K2_GetActorRotation` _output)))
    (:`Finished`
      (`KismetSystemLibrary.PrintString` "Impluse Added to Forcefield, sending it flying!!" true true (struct :`G` 0.061501 :`B` 1.0 :`A` 1.0) 6.0)
      (`self.Change Getting Knocked`)
      (`self.Feel Free to Knockback`))))

(event `Chase Player`)

(event `self.ReceiveBeginPlay`
  ;[1 1 1] Set Player Character for Reference later
  (bind _outactors (`GameplayStatics.GetAllActorsOfClass` "/Game/ThirdPersonBP/Blueprints/BP_MemeMan.BP_MemeMan_C"))
  (set `self.3rdPersonRef` (`|GetArrayItem` _outactors))
  (bind _outactors_2 (`GameplayStatics.GetAllActorsOfClass` "/Game/BluePrints/BP_ForcefieldKnockbackDirector.BP_ForcefieldKnockbackDirector_C"))
  (set `self.ForcefieldKnockback` (`self.K2_GetActorLocation` (`|GetArrayItem` _outactors_2))))

(event `Change Getting Knocked`
  ;[1 1 1] Change "Getting Knocked"
  (if (`self.GettingKnocked`)
    (set `self.GettingKnocked` false)
    (else
      (set `self.GettingKnocked` true))))

(event `Feel Free to Knockback`
  (bind _3rdpersonref (`self.3rdPersonRef`))
  (goto _label :!via `Reset`))

(event `self.ReceiveTick`
  (params (DeltaSeconds :type "Float (single-precision)"))
  (bind _3rdpersonref (`self.3rdPersonRef`))
  (if (`self.GettingKnocked`)
    (`/Engine/EditorBlueprintResources/StandardMacros.DoOnce` false :!label _label
      (:`Completed`
        (`self.Knock ForceField`)
        ;[1 1 1] Used if it's the last QTE
        (if (`KismetSystemLibrary.IsValid` _3rdpersonref)
          (`self.Speed Doer` (`/Game/ThirdPersonBP/Blueprints/BP_MemeMan.PlayerScore` _3rdpersonref)))))
    (else
      ;[1 1 1] Forcefeild gives chase if controller 3rd Person Character
      (if (== (`self.3rdPersonRef`) (`Controller.K2_GetPawn` (`GameplayStatics.GetPlayerController` 0)))
        ;[1 1 1] Chase Player
        (bind _asbp_meme_man (cast `/Game/ThirdPersonBP/Blueprints/BP_MemeMan` (`GameplayStatics.GetPlayerCharacter` 0))
          (:`then`
            (`self.K2_SetActorRotation` (`KismetMathLibrary.RInterpTo` (`self.K2_GetActorRotation` self) (`KismetMathLibrary.FindLookAtRotation` (`self.K2_GetActorLocation` self) (`self.K2_GetActorLocation` _asbp_meme_man)) 1.0 1.0))
            (`self.AddMovementInput` (`self.GetActorForwardVector` self)))
          (:`CastFailed`
            (`KismetSystemLibrary.PrintString` "Cast failed to ThirdPersonCharacter in BP_AIForcefield")))))))

(event `Speed Doer`
  (params (`What Speed?` :type "Float (double-precision)"))
  ;[1 1 1] Forcefield increase speed
  (if (>= `What Speed?` 500.0)
    (if (>= `What Speed?` 1000.0)
      (if (>= `What Speed?` 1500.0)
        (`/Engine/EditorBlueprintResources/StandardMacros.DoOnce` false
          (:`Completed`
            (bind (_direction _amount_to_speed) (`Timeline|1500 to 2000` :!via `PlayFromStart`)
              (:`Update`
                (set `FloatingPawnMovement.MaxSpeed` _amount_to_speed (`self.FloatingPawnMovement`)))
              (:`Finished`
                (`KismetSystemLibrary.PrintString` "Speed increased from 1000 to 1500" true true (struct :`G` 1.0 :`B` 0.197433 :`A` 1.0) 5.0)))))
        (else
          (`/Engine/EditorBlueprintResources/StandardMacros.DoOnce` false
            (:`Completed`
              (bind (_direction_2 _amount_of_speed) (`Timeline|From 1000 to 1500` :!via `PlayFromStart`)
                (:`Update`
                  (set `FloatingPawnMovement.MaxSpeed` _amount_of_speed (`self.FloatingPawnMovement`)))
                (:`Finished`
                  (`KismetSystemLibrary.PrintString` "Speed increased from 1000 to 1500" true true (struct :`G` 1.0 :`B` 0.197433 :`A` 1.0) 5.0)))))))
      (else
        (`/Engine/EditorBlueprintResources/StandardMacros.DoOnce` false
          (:`Completed`
            (bind (_direction_3 _newtrack_0) (`Timeline|From 500 to 1000` :!via `PlayFromStart`)
              (:`Update`
                (set `FloatingPawnMovement.MaxSpeed` _newtrack_0 (`self.FloatingPawnMovement`)))
              (:`Finished`
                (`KismetSystemLibrary.PrintString` "Speed increased from 500 to 1000" true true (struct :`R` 1.0 :`G` 0.13186 :`A` 1.0) 5.0)))))))))

(fn `UserConstructionScript`)