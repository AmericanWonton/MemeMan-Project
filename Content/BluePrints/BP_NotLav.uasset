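; BP_NotLav is a lava-style kill volume that kills and respawns the player.
; On BeginPlay it caches the world location of its PlayerRespawn component as the respawn point.
; When an actor tagged PlayerCharacter overlaps its Box, it passes that point to the first BP_MemeMan's QTEFailedKnockingMemeMan.
; It then calls DeadRespawn on player controller 0, cast to BP_ThePlayerController, passing itself.
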(event `self.ReceiveBeginPlay`
  ;[1 1 1] Respawn Location Set
  (set `self.Respawn Location` (`SceneComponent.K2_GetComponentLocation` (`self.PlayerRespawn`))))

(event `self.Box.OnComponentBeginOverlap`
  (params (OverlappedComponent :type "PrimitiveComponent Object Reference") (OtherActor :type "Actor Object Reference") (OtherComp :type "PrimitiveComponent Object Reference") (OtherBodyIndex :type Integer) (bFromSweep :type Boolean) (SweepResult :type "HitResult Structure (by ref)"))
  ;[1 1 1] Lava death, takes away visibility and input and then  sets it back after three seconds.
  (if (`self.ActorHasTag` OtherActor "PlayerCharacter")
    (`KismetSystemLibrary.PrintString` "P1 is dead and respawning.")
    (bind _outactors (`GameplayStatics.GetAllActorsOfClass` "/Game/ThirdPersonBP/Blueprints/BP_MemeMan.BP_MemeMan_C"))
    (`/Game/ThirdPersonBP/Blueprints/BP_MemeMan.QTE Failed, Knocking Meme Man!` (`|GetArrayItem` _outactors) (`self.Respawn Location`))
    (bind _asbp_the_player_controller (cast `/Game/Utility/BP_ThePlayerController` (`GameplayStatics.GetPlayerController` 0))
      (:`then`
        (`/Game/Utility/BP_ThePlayerController.Dead Respawn!` _asbp_the_player_controller self))
      (:`CastFailed`
        (`KismetSystemLibrary.PrintString` "Cast failed to BP_PlayerController in BP_Not Lav")))))

(fn `UserConstructionScript`)