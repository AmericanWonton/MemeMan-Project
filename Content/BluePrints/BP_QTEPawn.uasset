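; BP_QTEPawn is a trigger pawn that starts a quick-time event when the player character overlaps its sphere.
; A timeline slows global time, then the player controller enters QTE mode and the HUD shows a random QTE widget.
; Winning restores time and control, awards score, signals the forcefield and captain actors, then destroys the pawn.
; Losing zeroes the score, knocks BP_MemeMan to a fail location and resets its DoOnce for retry.
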(event `InputAction|Pause Game`
  (params (Key :type "Key Structure"))
  ;[1 1 1] Used to Pause all Interactable Widgets
  (:`Pressed`
    (bind _outactors (`GameplayStatics.GetAllActorsOfClass` "/Game/ThirdPersonBP/Blueprints/BP_MemeMan.BP_MemeMan_C"))
    (`/Game/ThirdPersonBP/Blueprints/BP_MemeMan.Pause Game` (`|GetArrayItem` _outactors))))

(event `self.Sphere.OnComponentBeginOverlap`
  (params (OverlappedComponent :type "PrimitiveComponent Object Reference") (OtherActor :type "Actor Object Reference") (OtherComp :type "PrimitiveComponent Object Reference") (OtherBodyIndex :type Integer) (bFromSweep :type Boolean) (SweepResult :type "HitResult Structure (by ref)"))
  ;[1 1 1] Activate QTE Event when Overlapped
  (if (`self.ActorHasTag` OtherActor "PlayerCharacter")
    (`KismetSystemLibrary.PrintString` "Doing QTE!" true true (struct :`R` 0.918744 :`G` 0.202529 :`B` 1.0 :`A` 1.0) 4.0)
    ;;[1 1 1] Used later in the HUD
    (set `self.Is Possesed?` true)
    ;[1 1 1] Used for typing input(May not need for phones)
    (bind _asbp_the_player_controller (cast `/Game/Utility/BP_ThePlayerController` (`GameplayStatics.GetPlayerController` 0))
      (:`then`
        (`/Game/Utility/BP_ThePlayerController.Allow Controls for QTE` _asbp_the_player_controller)
        ;;[1 1 1] Used to reset your failures
        (set `self.Score Amount` 500.0)
        (bind (_direction _timeslow) (`Timeline|Time SloMO` :!via `PlayFromStart`)
          (:`Update`
            (`GameplayStatics.SetGlobalTimeDilation` _timeslow))
          (:`Finished`
            (bind _asbp_the_player_controller_2 (cast `/Game/Utility/BP_ThePlayerController` (`GameplayStatics.GetPlayerController` 0))
              (:`then`
                (`/Game/Utility/BP_ThePlayerController.QTE Event` _asbp_the_player_controller_2 self)
                (`self.Do Random QTE`))
              (:`CastFailed`
                (`KismetSystemLibrary.PrintString` "Cast failed to BP_PlayerController in BP_WTEPawn"))))))
      (:`CastFailed`
        (`KismetSystemLibrary.PrintString` "Cast failed to BP Player controller in BP_QTEPawn")))
    (else
      (`KismetSystemLibrary.PrintString` "QTE Colliding with Somethign Else" true true (struct :`R` 1.0 :`G` 0.261035 :`A` 1.0) 1.0))))

(event `Do Random QTE`
  ;[1 1 1] Send and Create Widget
  (bind _output_get (set `self.Which QTE Event?` (`KismetMathLibrary.RandomIntegerInRange` 0 1)))
  (bind _asbp_the_hud (cast `/Game/Utility/BP_TheHUD` (`PlayerController.GetHUD` (`GameplayStatics.GetPlayerController` 0)))
    (:`then`
      (`/Game/Utility/BP_TheHUD.Add new QTE Widget` _asbp_the_hud _output_get))
    (:`CastFailed`
      (`KismetSystemLibrary.PrintString` "Cast to HUD failed in W_QTEQUEstion 1"))))

(event `Key|SpaceBar`
  (params (Key :type "Key Structure"))
  ;[1 1 1] The QTE Button
  (:`Pressed`
    (bind _output_get (set `self.Button Presses!` (+ (`self.Button Presses!`) 1)))
    (if (not (>= _output_get 50))
      (`KismetSystemLibrary.PrintString` (`KismetStringLibrary.Concat_StrStr` "You have " (`KismetStringLibrary.Conv_IntToString` _output_get) " button presses!")))))

(event `Done with this QTE(Win)`
  (params (`Won or Lost?` :type Boolean))
  ;[1 1 1] Win or lose score to pass to player
  (`/Engine/EditorBlueprintResources/StandardMacros.DoOnce` false
    (:`Completed`
      (set `self.Score Amount` 500.0)
      (`KismetSystemLibrary.PrintString` "QTE Complete, you won!")
      ;[1 1 1] Move the Forcefield
      (bind _outactors (`GameplayStatics.GetAllActorsOfClass` "/Game/BluePrints/AI_Enemies/BP_AIForceField.BP_AIForceField_C"))
      (bind (_direction _timeslow) (`Timeline|Un-SloMo` :!via `PlayFromStart`)
        (:`Update`
          (`GameplayStatics.SetGlobalTimeDilation` _timeslow))
        (:`Finished`
          ;[1 1 1] Give Control Back to Player
          (bind _asbp_the_player_controller (cast `/Game/Utility/BP_ThePlayerController` (`GameplayStatics.GetPlayerController` 0))
            (:`then`
              (`/Game/Utility/BP_ThePlayerController.QTE Exit Transition` _asbp_the_player_controller)
              (`/Game/Utility/BP_ThePlayerController.take away Controls for QTE` _asbp_the_player_controller)
              (set `self.Button Presses!` 0)
              ;[1 1 1] Set Score in Widget and PlayerHCaracter from BP_TheHud
              (bind _asbp_the_hud (cast `/Game/Utility/BP_TheHUD` (`PlayerController.GetHUD` (`GameplayStatics.GetPlayerController` 0)))
                (:`then`
                  (`/Game/Utility/BP_TheHUD.Set Score Widget` _asbp_the_hud (`self.Score Amount`))
                  (`/Game/Utility/BP_TheHUD.Player Score Setter` _asbp_the_hud (`self.Score Amount`))
                  ;;[1 1 1] If player succeeded in winning this QTE
                  (bind _outactors_2 (`GameplayStatics.GetAllActorsOfClass` "/Game/BluePrints/BP_CaptainWinState.BP_CaptainWinState_C"))
                  (message `/Game/Interfaces/BPI_DeadQTE.Hey, Dead QTE` (`|GetArrayItem` _outactors_2))
                  (`/Game/BluePrints/AI_Enemies/BP_AIForceField.Change Getting Knocked` (`|GetArrayItem` _outactors))
                  (set `self.Is Possesed?` false)
                  (`self.K2_DestroyActor`))
                (:`CastFailed`
                  (`KismetSystemLibrary.PrintString` "Cast failed to BP_The HUD in BP_Time Decreaser"))))
            (:`CastFailed`
              (`KismetSystemLibrary.PrintString` "Cast failed to BP_PlayerController in BP_WTEPawn"))))))))

(event `self.ReceiveBeginPlay`
  ;[1 1 1] Set Failed Spawn Location for faileing this QTE
  (set `self.Failed Spawn Locaiton` (`SceneComponent.K2_GetComponentLocation` (`self.FailedSpawnLocal`))))

(event `Done with this QTE (Lost)`
  (params (NewParam :type Boolean))
  (set `self.Score Amount` 0.0)
  (`/Engine/EditorBlueprintResources/StandardMacros.DoOnce` false :!label _label
    (:`Completed`
      (`KismetSystemLibrary.PrintString` "QTE Complete, you failed!")
      (bind (_direction _timeslow) (`Timeline|Timeline_0` :!via `PlayFromStart`)
        (:`Update`
          (`GameplayStatics.SetGlobalTimeDilation` _timeslow))
        (:`Finished`
          (bind _asbp_the_player_controller (cast `/Game/Utility/BP_ThePlayerController` (`GameplayStatics.GetPlayerController` 0))
            (:`then`
              (`/Game/Utility/BP_ThePlayerController.QTE Exit Transition` _asbp_the_player_controller)
              (`/Game/Utility/BP_ThePlayerController.take away Controls for QTE` _asbp_the_player_controller)
              (set `self.Button Presses!` 0)
              (bind _asbp_the_hud (cast `/Game/Utility/BP_TheHUD` (`PlayerController.GetHUD` (`GameplayStatics.GetPlayerController` 0)))
                (:`then`
                  (`/Game/Utility/BP_TheHUD.Set Score Widget` _asbp_the_hud (`self.Score Amount`))
                  (`/Game/Utility/BP_TheHUD.Player Score Setter` _asbp_the_hud (`self.Score Amount`))
                  (set `self.Is Possesed?` false)
                  ;[1 1 1] Catapult Meme Man to a safe distance
                  (bind _outactors (`GameplayStatics.GetAllActorsOfClass` "/Game/ThirdPersonBP/Blueprints/BP_MemeMan.BP_MemeMan_C"))
                  (`/Game/ThirdPersonBP/Blueprints/BP_MemeMan.QTE Failed, Knocking Meme Man!` (`|GetArrayItem` _outactors) (`self.Failed Spawn Locaiton`))
                  ;[1 1 1] Make sure the "Do once can be alled again"
                  (`self.Rest the Failure`))
                (:`CastFailed`
                  (`KismetSystemLibrary.PrintString` "Cast failed to BP_The HUD in BP_Time Decreaser"))))
            (:`CastFailed`
              (`KismetSystemLibrary.PrintString` "Cast failed to BP_PlayerController in BP_WTEPawn"))))))))

(event `Rest the Failure`
  (goto _label :!via `Reset`))

(fn `UserConstructionScript`)