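; BP_CaptainWinState tracks the level's remaining QTEs and handles the game-over sequence.
; After a startup delay it counts BP_QTEPawns and caches the end camera; each DeadQTE event decrements the count, declaring a win at zero.
; WinStateShower switches to that camera, then once destroys BP_MemeMan, has BP_TheHUD show the results widget, and saves score plus time bonus through BP_TheGameMode.
; An older save-and-quit chain remains unconnected.
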(event `self.ReceiveBeginPlay`
  ;[1 1 1] Set number of QTE's to finish
  (`KismetSystemLibrary.Delay` 3.0)
  (bind _outactors (`GameplayStatics.GetAllActorsOfClass` "/Game/BluePrints/BP_QTEPawn.BP_QTEPawn_C"))
  (set `self.Number of QTE's` (`KismetArrayLibrary.Array_Length` _outactors))
  ;[1 1 1] Sets win/Lose Camera for Later
  (bind _outactors_2 (`GameplayStatics.GetAllActorsOfClass` "/Game/BluePrints/BP_CaptainWinState_Camera.BP_CaptainWinState_Camera_C"))
  (set `self.Camera Ref` (`|GetArrayItem` _outactors_2)))

(event `/Game/Interfaces/BPI_DeadQTE.Hey, Dead QTE`
  ;[1 1 1] A Win or "Still to Go" State
  (bind _output_get (set `self.Number of QTE's` (- (`self.Number of QTE's`) 1)))
  (if (== _output_get 0)
    (set `self.You Won` true)
    (`self.Win State Shower`)
    (else
      (`KismetSystemLibrary.PrintString` (`KismetStringLibrary.Concat_StrStr` "There's still " (`KismetStringLibrary.Conv_IntToString` _output_get) " QTE's to go!") true true (struct :`R` 1.0 :`G` 0.927169 :`B` 0.058036 :`A` 1.0) 4.0))))

(event `Win State Shower`
  ;[1 1 1] Win/Lose State Business
  ;;[1 1 1] Go 2 Game Over Camera
  (bind _asbp_the_player_controller (cast `/Game/Utility/BP_ThePlayerController` (`GameplayStatics.GetPlayerController` 0))
    (:`then`
      (`/Game/Utility/BP_ThePlayerController.Game Over Camera` _asbp_the_player_controller (`self.Camera Ref`))
      (`/Engine/EditorBlueprintResources/StandardMacros.DoOnce` false
        (:`Completed`
          ;;[1 1 1] Destroy Actor for BP_TheHUD to get score
          (bind _outactors (`GameplayStatics.GetAllActorsOfClass` "/Game/ThirdPersonBP/Blueprints/BP_MemeMan.BP_MemeMan_C"))
          (bind _output (`|GetArrayItem` _outactors))
          (`/Game/ThirdPersonBP/Blueprints/BP_MemeMan.Destroy Me Info` _output)
          (`self.SetLifeSpan` _output 0.5)
          ;;[1 1 1] Create Game Over Widget
          (bind _asbp_the_hud (cast `/Game/Utility/BP_TheHUD` (`PlayerController.GetHUD` (`GameplayStatics.GetPlayerController` 0)))
            (:`then`
              (bind _timer_value (`/Game/Utility/BP_TheHUD.Timer Value` _asbp_the_hud))
              (`/Game/Utility/BP_TheHUD.Game Over Widget Creation` _asbp_the_hud (`self.Number of QTE's`) _timer_value (`self.You Won`))
              ;;[1 1 1] Set and Save Final Score
              (bind _output_get (set `self.Time Left` _timer_value))
              (bind _output_get_2 (set `self.Final Score` (+ (`self.PlayerScore`) (* _output_get 100.0))))
              (`KismetSystemLibrary.PrintString` "Game Over, you win!" true true (struct :`R` 0.188427 :`G` 1.0 :`A` 1.0) 10.0)
              (bind _asbp_the_game_mode (cast `/Game/Utility/BP_TheGameMode` (`GameplayStatics.GetGameMode`))
                (:`then`
                  (`/Game/Utility/BP_TheGameMode.Save and Load Player Score` _asbp_the_game_mode _output_get_2 (`self.What Level`)))
                (:`CastFailed`
                  (`KismetSystemLibrary.PrintString` "Cast failed to BP_TheGameMode in BP_CaptainWinState"))))
            (:`CastFailed`
              (`KismetSystemLibrary.PrintString` "Cast failed to BP_TheHUd in BP_CaptainWinState"))))))
    (:`CastFailed`
      (`KismetSystemLibrary.PrintString` "Cast failed to Playercontrolller in BP_Captain Win State"))))

(fn `UserConstructionScript`)